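; BP_Blocks is an actor that forms a grid of breakable blocks hit by BP_Ball.
; The construction script adds static mesh components in rows and columns sized by X and Y and spaced by Padding.
; A ball hit turns a non-red block red, while a hit on a red block destroys that component and occasionally spawns a BP_Bonus at its location.
; The material itself serves as the damage state, and SetDamage is empty.
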(event Collision|EventHit
  (params (MyComp :type Primitive%20Component%20Object%20Reference) (Other :type Actor%20Object%20Reference) (OtherComp :type Primitive%20Component%20Object%20Reference) (bSelfMoved :type Boolean) (HitLocation :type Vector :default "0, 0, 0") (HitNormal :type Vector :default "0, 0, 0") (NormalImpulse :type Vector :default "0, 0, 0") (Hit :type Hit%20Result%20Structure%20%28by%20ref%29))
  (bind _red (Variables|Default|GetRed))
  ;[1 0.3497 0.9435] DESTROY COMPONENTS
  (Utilities|Casting|CastToBP_Ball Other)
  (Variables|Default|SetBonusLocation (Transformation|GetWorldLocation MyComp))
  (if (== (Rendering|Material|GetMaterial MyComp 0) _red)
    (Components|DestroyComponent MyComp)
    ;[0 0.886 1] Spawn Bonus
    (if (Math|Random|RandomBoolwithWeight 0.2)
      (Game|SpawnActorfromClass "/Game/Blueprints/BP_Bonus.BP_Bonus_C" (Math|Transform|MakeTransform (Variables|Default|GetBonusLocation) "0, 0, 0" "1,1,1") "AlwaysSpawn" 0 0))
    (else
      (Rendering|Material|SetMaterial MyComp 0 _red))))

(fn ConstructionScript
  (for _index (range 0 (Variables|Default|GetX))
    (for _index_2 (range 0 (Variables|Default|GetY))
      (AddComponent|AddStaticMeshComponent false (Math|Transform|MakeTransform (Math|Vector|MakeVector (Math|Conversions|ToFloat(Integer) (* _index (Variables|Default|GetPadding))) (Math|Conversions|ToFloat(Integer) (* _index_2 (Variables|Default|GetPadding))) 0.0))))))

(fn SetDamage)