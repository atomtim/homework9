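; BP_Bonus is a moving pickup that grants an extra ball when a BP_Pawn catches it.
; Each tick it moves along Direction at Speed with a frame-rate independent, swept offset.
; On overlap with a BP_Pawn it fires the OnCatch dispatcher, spawns a BP_Ball at its Sphere's location regardless of collision, and destroys itself.
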(event Collision|EventActorBeginOverlap
  (params (OtherActor :type Actor%20Object%20Reference))
  (Utilities|Casting|CastToBP_Pawn OtherActor)
  (Default|CallOnCatch)
  (Game|SpawnActorfromClass "/Game/Blueprints/BP_Ball.BP_Ball_C" (Math|Conversions|ToTransform(Vector) (Transformation|GetWorldLocation (Variables|Default|GetSphere))) "AlwaysSpawn" 0 0)
  (Actor|DestroyActor))

(event EventTick
  (params (DeltaSeconds :type Float%20%28single-precision%29))
  (Transformation|AddActorWorldOffset (* (* (Variables|Default|GetDirection) (Variables|Default|GetSpeed)) DeltaSeconds) true))

(fn ConstructionScript)