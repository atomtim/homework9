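; BP_Ball is a bouncing ball actor that moves at a set speed along a direction and dies in kill zones.
; Each Tick sweeps it forward by Direction, Speed and delta time, without using physics forces.
; On a blocking hit, SetReflection derives a new direction from the hit normal's X and Y.
; Overlapping a KillZVolume fires the OnDead dispatcher, then destroys the ball.
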(event Collision|EventActorBeginOverlap
  (params (OtherActor :type Actor%20Object%20Reference))
  ;[1 0.0304 0] KILL ZONE || SPAWN BALLS || LIFES
  (Utilities|Casting|CastToKillZVolume OtherActor)
  (Default|CallOnDead)
  (Actor|DestroyActor))

(event EventTick
  (params (DeltaSeconds :type Float%20%28single-precision%29))
  ;[1 0.9104 0] SPEED & DIRECTION
  (bind _sweephitresult (Transformation|AddActorWorldOffset (* (* (Variables|Default|GetDirection) (Variables|Default|GetSpeed)) DeltaSeconds) true))
  (if (.bBlockingHit (Collision|BreakHitResult _sweephitresult))
    (CallFunction|SetReflection "0, 0, 0" (.Normal (Collision|BreakHitResult _sweephitresult)))))

(fn ConstructionScript)

(fn SetReflection
  (params (SurfaceNormal :type Vector) (InVec :type Vector))
  (bind (_x _y) (Math|Vector|BreakVector InVec))
  (Variables|Default|SetDirection (Math|Vector|GetReflectionVector (Variables|Default|GetDirection) (Math|Vector|MakeVector _x _y 0.0))))